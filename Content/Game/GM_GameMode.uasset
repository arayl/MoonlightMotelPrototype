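; Game mode for a ghost hotel management game, holding money, clock, cleaning upgrades and cleaner counts and pushing them to the main UI widget.
; Two looping timers drive it: one advances the clock and checks room checkouts, the other collects income from occupied rooms and rolls ghost arrivals with a randomized cooldown.
; Occupied rooms raise arrival chance up to a level cap.
; Clicking a waiting ghost, then a free room widget, checks it in.
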(event Custom|ReceiveTip
  (params (TipAmount :type Integer))
  (Variables|Default|SetPlayerDollars (+ (Variables|Default|GetPlayerDollars) TipAmount))
  (CallFunction|UpdateDollars)
  (CallFunction|AddXp))

(event Custom|UpdateTimer
  (if (== (Variables|Default|GetTimeMinutes) 59)
    (if (== (Variables|Default|GetTimeHours) 23)
      (Variables|Default|SetTimeHours 0)
      (Variables|Default|SetTimeMinutes 0)
      (else
        (Math|Integer|IncrementInt (Variables|Default|GetTimeHours)
          (:%20%20
            (Variables|Default|SetTimeMinutes 0)))))
    (else
      (Math|Integer|IncrementInt (Variables|Default|GetTimeMinutes)
        (:%20%20
          _))))
  (Default|UpdateTime (Variables|Default|GetMainUI) (Variables|Default|GetTimeHours) (Variables|Default|GetTimeMinutes))
  (bind _foundwidgets (Widget|GetAllWidgetsOfClass "/Game/UI/UW_Room.UW_Room_C" false))
  (for _array_element _foundwidgets
    (Default|CheckifIsCheckoutTime _array_element (Variables|Default|GetTimeHours) (Variables|Default|GetTimeMinutes))))

(event Custom|AddCleaner
  (Math|Integer|IncrementInt (Variables|Default|GetNumberOfCleaners)
    (:%20%20
      (Math|Integer|IncrementInt (Variables|Default|GetInactiveCleaners)
        (:%20%20
          (Default|SetCleanersText (Variables|Default|GetMainUI) (Variables|Default|GetNumberOfCleaners) (Variables|Default|GetActiveCleaners)))))))

(event Custom|OccupyCleaner
  (Math|Integer|IncrementInt (Variables|Default|GetActiveCleaners)
    (:%20%20
      (Math|Integer|DecrementInt (Variables|Default|GetInactiveCleaners)
        (:%20%20
          (Default|SetCleanersText (Variables|Default|GetMainUI) (Variables|Default|GetNumberOfCleaners) (Variables|Default|GetActiveCleaners)))))))

(event Custom|FreeCleaner
  (Math|Integer|IncrementInt (Variables|Default|GetInactiveCleaners)
    (:%20%20
      (Math|Integer|DecrementInt (Variables|Default|GetActiveCleaners)
        (:%20%20
          (Default|SetCleanersText (Variables|Default|GetMainUI) (Variables|Default|GetNumberOfCleaners) (Variables|Default|GetActiveCleaners)))))))

(event Custom|GhostArrivalCheck
  (bind _ghostarrivalcooldownmodifierpercentage (Variables|Default|GetGhostArrivalCooldownModifierPercentage))
  (bind _ghostarrivalcooldownrate (Variables|Default|GetGhostArrivalCooldownRate))
  (bind _returnvalue (Math|Random|RandomIntegerinRange 0 _ghostarrivalcooldownmodifierpercentage))
  (bind _returnvalue_2 (/ _returnvalue 100))
  (bind _returnvalue_3 (* _ghostarrivalcooldownrate _returnvalue_2))
  (if (>= (Variables|Default|GetChanceOfGhostArriving) (Math|Random|RandomFloatinRange 0.0 1e+02))
    (if (== (Math|Random|RandomIntegerinRange 0 1) 0)
      (Variables|Default|SetGhostArrivalCooldown (Math|Float|Round (+ (Variables|Default|GetGhostArrivalCooldownRate) _returnvalue_3)))
      (else
        (Variables|Default|SetGhostArrivalCooldown (Math|Float|Round (- (Variables|Default|GetGhostArrivalCooldownRate) _returnvalue_3)))))
    (CallFunction|GhostArrival)))

(event Custom|GhostArrival
  (Default|AddGhosttoWaitingRoom (Variables|Default|GetMainUI)))

(event Custom|GhostClickAttempt
  (params (Ghost :type UW%20Ghost%20Object%20Reference))
  (bind _output_get (Variables|Default|SetGhostClicked Ghost))
  (Default|SetasSelected _output_get))

(event Custom|ClickRoom
  (params (Room :type UW%20Room%20Object%20Reference))
  (if (!= (Variables|Default|GetGhostClicked) 0)
    (bind _isoccupied (Default|GetIsOccupied Room))
    (if (not _isoccupied)
      (bind _desiredtime (Default|GetDesiredTime (Variables|Default|GetGhostClicked)))
      (Default|AssignGhost Room _desiredtime)
      (Default|SetCheckinTime Room (Variables|Default|GetTimeHours) (Variables|Default|GetTimeMinutes))
      (Default|RemovefromScreen (Variables|Default|GetGhostClicked))
      (Variables|Default|SetGhostClicked 0))))

(event Custom|GameTick
  (Utilities|FlowControl|Sequence
    (:then_0
      (if (<= (Variables|Default|GetGhostArrivalCooldown) 0)
        (CallFunction|GhostArrivalCheck)
        (else
          (Math|Integer|DecrementInt (Variables|Default|GetGhostArrivalCooldown)))))
    (:then_1
      (bind _foundwidgets (Widget|GetAllWidgetsOfClass "/Game/UI/UW_Room.UW_Room_C" false))
      (for _array_element _foundwidgets
        (bind _isoccupied (Default|GetIsOccupied _array_element))
        (if _isoccupied
          (bind _minuterate (Default|GetMinuteRate _array_element))
          (Variables|Default|SetTickMoneyUpdate (+ (Variables|Default|GetTickMoneyUpdate) _minuterate))
          (if (< (Variables|Default|GetChanceOfGhostArriving) (Variables|Default|GetMaxGhostChanceForLevel))
            (if (> (Variables|Default|GetChanceOfGhostArriving) (Variables|Default|GetMaxGhostChanceForLevel))
              (Variables|Default|SetChanceOfGhostArriving (Variables|Default|GetMaxGhostChanceForLevel)))
            (Variables|Default|SetChanceOfGhostArriving (+ (Variables|Default|GetChanceOfGhostArriving) (Variables|Default|GetGhostChanceTickIncrease))))))
      (Variables|Default|SetPlayerDollars (+ (Variables|Default|GetPlayerDollars) (Variables|Default|GetTickMoneyUpdate)))
      (Variables|Default|SetTickMoneyUpdate 0)
      (CallFunction|UpdateDollars))))

(event Custom|UpdateDollars
  (Default|SetDollarAmountText (Variables|Default|GetMainUI) (Variables|Default|GetPlayerDollars)))

(event Custom|UpgradeCleaningPower
  (if (>= (Variables|Default|GetPlayerDollars) (Variables|Default|GetCleaningUpgradeCost))
    (Variables|Default|SetPlayerDollars (- (Variables|Default|GetPlayerDollars) (Variables|Default|GetCleaningUpgradeCost)))
    (CallFunction|UpdateDollars)
    (Math|Integer|IncrementInt (Variables|Default|GetCleaningLevel)
      (:%20%20
        (Variables|Default|SetCleaningUpgradeCostPerLevel (+ (Variables|Default|GetCleaningUpgradeCostPerLevel) (* (/ (Variables|Default|GetCleaningUpgradeCostPerLevel) 100) (Variables|Default|GetCleaningUpgradeCostPercentageIncrease))))
        (Variables|Default|SetCleaningUpgradeCost (* (Variables|Default|GetCleaningLevel) (Variables|Default|GetCleaningUpgradeCostPerLevel)))
        (Variables|Default|SetPlayerCleanSpeed (+ (Variables|Default|GetPlayerCleanSpeed) (Variables|Default|GetCleaningPowerUpgradeAmount)))))))

(event Custom|AddXp
  (Default|AddXP (Variables|Default|GetMainUI) 1e+01))

(event EventBeginPlay
  (Variables|Default|SetCleaningLevel 1)
  (Variables|Default|SetCleaningUpgradeCostPerLevel 500)
  (Variables|Default|SetCleaningUpgradeCost (* (Variables|Default|GetCleaningLevel) (Variables|Default|GetCleaningUpgradeCostPerLevel)))
  (bind _returnvalue (UserInterface|CreateWidget "/Game/UI/UW_MainUI.UW_MainUI_C"))
  (Variables|Default|SetMainUI _returnvalue)
  (UserInterface|Viewport|AddtoViewport (Variables|Default|GetMainUI) 0)
  (Utilities|Time|SetTimerbyEvent (delegate Custom|UpdateTimer) (Variables|Default|GetTimeToUpdateTimer) true)
  (Utilities|Time|SetTimerbyEvent (delegate Custom|GameTick) (Variables|Default|GetGameTickTime) true))

(fn ConstructionScript)

(fn GetPlayerCleanSpeed
  (return (Variables|Default|GetPlayerCleanSpeed)))

(fn GetCleaningLevelUpgradeCost
  (return (Variables|Default|GetCleaningUpgradeCost)))

(fn CheckforMoneyandCharge
  (params (AmountToCheck :type Integer))
  (if (>= (Variables|Default|GetPlayerDollars) AmountToCheck)
    (LocalVariables|SetPlayerWasCharged true)
    (Variables|Default|SetPlayerDollars (- (Variables|Default|GetPlayerDollars) AmountToCheck))
    (CallFunction|UpdateDollars)
    (else
      (LocalVariables|SetPlayerWasCharged false)))
  (return (LocalVariables|GetPlayerWasCharged)))